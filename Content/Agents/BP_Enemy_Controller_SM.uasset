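; AI controller for enemy agents that runs a state machine component, giving its blackboard the pawn and controller before starting it.
; Perception updates toggle the seen player, setting or clearing blackboard data, with the search location lerped most of the way toward the player.
; A cancellable scan timer promotes the seen player to attack target on completion.
; State changes pass the state name to the enemy pawn.
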(event `self.ReceiveBeginPlay`
  ; Begin Play
  (`|ExecutionSequence`
    (:`then_0`
      (bind _asbp_state_machine_blackboard (cast `/Game/AI/StateMachine/BP_StateMachine_Blackboard` (`RpStateMachineComponent.StateMachineBlackboard` (`self.StateMachineComponent`))))
      (`|ExecutionSequence`
        (:`then_0`
          (`/Game/AI/StateMachine/BP_StateMachine_Blackboard.SetAgent` _asbp_state_machine_blackboard (`self.K2_GetPawn`)))
        (:`then_1`
          (`/Game/AI/StateMachine/BP_StateMachine_Blackboard.SetController` _asbp_state_machine_blackboard self))))
    (:`then_1`
      (`RpStateMachineComponent.Start` (`self.StateMachineComponent`)))))

(event `StartScan`
  ; State Machine
  (bind _returnvalue (`KismetSystemLibrary.K2_SetTimerDelegate` (delegate `OnScanComplete`) 5.0))
  (set `self.ScanTimer` _returnvalue))

(event `OnScanComplete`
  ; State Machine
  (bind _returnvalue (`RpStateMachineComponent.GetContext` (`self.StateMachineComponent`) "/Game/AI/StateMachine/BP_StateMachine_Blackboard.BP_StateMachine_Blackboard_C"))
  (set `/Game/AI/StateMachine/BP_StateMachine_Blackboard.AttackTarget` (`self.SeenPlayer`) _returnvalue))

(event `EndScan`
  ; State Machine
  (`KismetSystemLibrary.K2_ClearAndInvalidateTimerHandle` (`self.ScanTimer`)))

(event `self.StateMachineComponent.OnStateChanged`
  (params (NewState :type String))
  ; State Machine
  (bind _asbp_enemy_pawn (cast `/Game/Agents/BP_Enemy_Pawn` (`self.K2_GetPawn`)))
  (`/Game/Agents/BP_Enemy_Pawn.SetStateName` _asbp_enemy_pawn (`KismetTextLibrary.Conv_StringToText` NewState)))

(event `self.AIPerception.OnPerceptionUpdated`
  (params (UpdatedActors :type "Array of Actor Object Reference (by ref)"))
  ; AI Perception
  (for _array_element UpdatedActors
    (bind _asbp_player (cast `/Game/Agents/BP_Player` _array_element))
    (`/Engine/EditorBlueprintResources/StandardMacros.IsValid` (`self.SeenPlayer`)
      (:`Is Valid`
        (`self.ClearSeenTarget`))
      (:`Is Not Valid`
        (`self.SetSeenTarget` _asbp_player)))))

(fn `ClearSeenTarget`
  (set `self.SeenPlayer` null)
  (bind _returnvalue (`RpStateMachineComponent.GetContext` (`self.StateMachineComponent`) "/Game/AI/StateMachine/BP_StateMachine_Blackboard.BP_StateMachine_Blackboard_C"))
  (set `/Game/AI/StateMachine/BP_StateMachine_Blackboard.WasSomethingSeen` false _returnvalue)
  (set `/Game/AI/StateMachine/BP_StateMachine_Blackboard.AttackTarget` null _returnvalue))

(fn `SetSeenTarget`
  (params (Target :type "/Game/Agents/BP_Player Object Reference"))
  (set `self.SeenPlayer` Target)
  (bind _returnvalue (`RpStateMachineComponent.GetContext` (`self.StateMachineComponent`) "/Game/AI/StateMachine/BP_StateMachine_Blackboard.BP_StateMachine_Blackboard_C"))
  (set `/Game/AI/StateMachine/BP_StateMachine_Blackboard.WasSomethingSeen` true _returnvalue)
  (set `/Game/AI/StateMachine/BP_StateMachine_Blackboard.SearchLocation` (`KismetMathLibrary.VLerp` (`self.K2_GetActorLocation` (`self.K2_GetPawn`)) (`self.K2_GetActorLocation` (`self.SeenPlayer`)) 0.8) _returnvalue))

(fn `UserConstructionScript`)