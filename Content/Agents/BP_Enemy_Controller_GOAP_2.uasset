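; AI controller that drives an enemy pawn with a GOAP component in a repeating reach-target loop.
; On BeginPlay it registers itself and its pawn in the GOAP blackboard, stores the starting transform, adds the ReachTarget goal, then plans and executes after a delay.
; When a goal is reached and ReachTarget is picked again, it teleports the pawn back, rewrites the base-state location fact and replans after a delay.
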(event `self.ReceiveBeginPlay`
  (bind _goapcomponent (`self.GOAPComponent`))
  (bind _returnvalue (`self.K2_GetPawn` self))
  ; Begin Play
  (`|ExecutionSequence`
    (:`then_0`
      (bind _returnvalue_2 (`RpGOAPComponent.GetContext` _goapcomponent "/Game/AI/GOAP/BP_GOAP_Blackboard.BP_GOAP_Blackboard_C"))
      (`/Game/AI/GOAP/BP_GOAP_Blackboard.SetController` _returnvalue_2 self)
      (`/Game/AI/GOAP/BP_GOAP_Blackboard.SetAgent` _returnvalue_2 _returnvalue)
      (set `self.StartingTransform` (`self.GetTransform` _returnvalue)))
    (:`then_1`
      (`RpGOAPComponent.AddGoal` _goapcomponent "/Game/AI/GOAP/Goals/BP_GOAP_Goal_ReachTarget.BP_GOAP_Goal_ReachTarget_C")
      (`RpGOAPComponent.PickGoal` _goapcomponent))
    (:`then_2`
      (`KismetSystemLibrary.Delay` 2.0)
      (`RpGOAPComponent.PlanAndExecute` _goapcomponent))))

(event `self.GOAPComponent.OnGoalReached`
  (params (Goal :type "RpGOAPGoal Object Reference"))
  (bind _goapcomponent (`self.GOAPComponent`))
  ; Loop goal.
  (bind _returnvalue (`RpGOAPComponent.PickGoal` _goapcomponent))
  (cast `/Game/AI/GOAP/Goals/BP_GOAP_Goal_ReachTarget` _returnvalue)
  (`self.ResetState`)
  (`KismetSystemLibrary.Delay` 2.0)
  (`RpGOAPComponent.PlanAndExecute` _goapcomponent))

(fn `ResetState`
  (bind _startingtransform (`self.StartingTransform`))
  (`self.K2_SetActorTransform` (`self.K2_GetPawn`) _startingtransform false true)
  (bind _returnvalue (`RpGOAPComponent.GetBaseState` (`self.GOAPComponent`)))
  (bind _returnvalue_2 (`BlueprintInstancedStructLibrary.MakeInstancedStruct` (make `RpVariantVector3` (.location _startingtransform))))
  (`RpGOAPState.SetFact` _returnvalue (`BlueprintGameplayTagLibrary.MakeLiteralGameplayTag` (struct :`TagName` "GOAP.PlayerState.Location")) (make `RpStateDescriptor` _returnvalue_2)))

(fn `UserConstructionScript`)