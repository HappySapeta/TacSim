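; Enemy AI controller that drives its pawn with a GOAP planner, looping through patrols to random nearby points.
; On begin play it binds the blackboard context, adds a Patrol goal and runs the planner.
; Each patrol resets the current-location fact and sets a new target, replanning after a random pause when reached.
; Functions to add or remove an Investigate goal for a seen player exist, but the perception event leaves them unwired.
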(event `self.ReceiveBeginPlay`
  (bind _goapcomponent (`self.GOAPComponent`))
  ; Begin Play
  (`|ExecutionSequence`
    (:`then_0`
      (bind _returnvalue (`RpGOAPComponent.GetContext` _goapcomponent "/Game/AI/GOAP/BP_GOAP_Blackboard.BP_GOAP_Blackboard_C"))
      (`/Game/AI/GOAP/BP_GOAP_Blackboard.SetController` _returnvalue self)
      (`/Game/AI/GOAP/BP_GOAP_Blackboard.SetAgent` _returnvalue (`self.K2_GetPawn` self)))
    (:`then_1`
      (bind _returnvalue_2 (`RpGOAPComponent.GetPlanner` _goapcomponent))
      (`RpGOAPPlanner.AddGoal` _returnvalue_2 "/Game/AI/GOAP/BP_GOAP_Goal_Patrol.BP_GOAP_Goal_Patrol_C")
      (`self.SetPatrolGoalData`))
    (:`then_2`
      (`KismetSystemLibrary.Delay` 1.0)
      (`RpGOAPComponent.PlanAndExecute` _goapcomponent))))

(event `self.AIPerception.OnPerceptionUpdated`
  (params (UpdatedActors :type "Array of Actor Object Reference (by ref)"))
  ; AI Perception
)

(event `self.GOAPComponent.OnGoalReached`
  (params (Goal :type "RpGOAPGoal Object Reference"))
  ; On Goal Reached - Loop through plan
  (`KismetSystemLibrary.Delay` (`KismetMathLibrary.RandomFloatInRange` 1.0 5.0))
  (`self.SetPatrolGoalData`)
  (`RpGOAPComponent.PlanAndExecute` (`self.GOAPComponent`)))

(fn `ClearSeenTarget`
  (`/Engine/EditorBlueprintResources/StandardMacros.IsValid` (`self.SeenPlayer`)
    (:`Is Valid`
      (set `self.SeenPlayer` null)
      (bind _returnvalue (`RpGOAPComponent.GetPlanner` (`self.GOAPComponent`)))
      (`RpGOAPPlanner.RemoveGoal` _returnvalue "/Game/AI/GOAP/BP_GOAP_Goal_Investigate.BP_GOAP_Goal_Investigate_C"))))

(fn `SetPatrolGoalData`
  (locals (CurrentLocationKey :type "GameplayTag Structure" :default (struct :`TagName` "GOAP.PlayerState.CurrentLocation")) (Planner :type "RpGOAPPlanner Object Reference") (MinPatrolRange :type "Float (double-precision)" :default 400.0) (MaxPatrolRange :type "Float (double-precision)" :default 700.0) (PatrolLocation :type "Vector Structure" :default (0.0 0.0 0.0)))
  (bind _returnvalue (`self.K2_GetActorLocation` (`self.K2_GetPawn`)))
  (bind _returnvalue_2 (`RpGOAPComponent.GetPlanner` (`self.GOAPComponent`)))
  (set `local.Planner` _returnvalue_2)
  (`|ExecutionSequence`
    (:`then_0`
      ; Reset current state
      (bind _returnvalue_3 (`BlueprintInstancedStructLibrary.MakeInstancedStruct` (make `RpVariantVector3` (`self.K2_GetActorLocation` (`self.K2_GetPawn`)))))
      (`RpGOAPState.SetFact` (`RpGOAPPlanner.StartingState` (`local.Planner`)) (`local.CurrentLocationKey`) (make `RpStateDescriptor` _returnvalue_3)))
    (:`then_1`
      ; Comment
      (set `local.PatrolLocation` (`KismetMathLibrary.MakeVector` (.x (+ _returnvalue (* (`KismetMathLibrary.RandomUnitVector`) (`KismetMathLibrary.RandomFloatInRange` (`local.MinPatrolRange`) (`local.MaxPatrolRange`))))) (.y (+ _returnvalue (* (`KismetMathLibrary.RandomUnitVector`) (`KismetMathLibrary.RandomFloatInRange` (`local.MinPatrolRange`) (`local.MaxPatrolRange`))))) (.z _returnvalue))))
    (:`then_2`
      ; Set goal
      (bind _returnvalue_4 (`RpGOAPPlanner.GetGoalOfType` (`local.Planner`) "/Game/AI/GOAP/BP_GOAP_Goal_Patrol.BP_GOAP_Goal_Patrol_C"))
      (`/Engine/EditorBlueprintResources/StandardMacros.IsValid` _returnvalue_4
        (:`Is Valid`
          (bind _returnvalue_5 (`BlueprintInstancedStructLibrary.MakeInstancedStruct` (make `RpVariantVector3` (`local.PatrolLocation`))))
          (`RpGOAPGoal.SetRequirement` _returnvalue_4 (`local.CurrentLocationKey`) (make `RpRequirementDescriptor` _returnvalue_5)))))
    (:`then_3`
      ; Comment
      (bind _returnvalue_6 (`RpGOAPComponent.GetContext` (`self.GOAPComponent`) "/Game/AI/GOAP/BP_GOAP_Blackboard.BP_GOAP_Blackboard_C"))
      (set `/Game/AI/GOAP/BP_GOAP_Blackboard.GoToLocation` (`local.PatrolLocation`) _returnvalue_6))))

(fn `SetSeenTarget`
  (params (Target :type "/Game/Agents/BP_Player Object Reference"))
  (`/Engine/EditorBlueprintResources/StandardMacros.IsValid` (`self.SeenPlayer`)
    (:`Is Not Valid`
      (bind _output_get (set `self.SeenPlayer` Target))
      (bind _returnvalue (`RpGOAPComponent.GetPlanner` (`self.GOAPComponent`)))
      (bind _returnvalue_2 (`RpGOAPPlanner.AddGoal` _returnvalue "/Game/AI/GOAP/BP_GOAP_Goal_Investigate.BP_GOAP_Goal_Investigate_C"))
      (bind _returnvalue_3 (`BlueprintInstancedStructLibrary.MakeInstancedStruct` (make `RpVariantVector3` (`self.K2_GetActorLocation` _output_get))))
      (`RpGOAPGoal.SetRequirement` _returnvalue_2 (`BlueprintGameplayTagLibrary.MakeLiteralGameplayTag` (struct :`TagName` "GOAP.PlayerState.CurrentLocation")) (make `RpRequirementDescriptor` _returnvalue_3)))))

(fn `UserConstructionScript`)