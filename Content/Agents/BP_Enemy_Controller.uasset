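; BP_Enemy_Controller is the controller for enemy agents that drives their behaviour through a state machine.
; On BeginPlay it casts the state machine's blackboard to BP_StateMachine_Blackboard, stores the controlled pawn as the agent and itself as the controller, then starts the machine.
; Start runs from its own sequence pin, so it fires even if the cast fails; Tick is unused.
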(event `self.ReceiveBeginPlay`
  (`|ExecutionSequence`
    (:`then_0`
      (bind _asbp_state_machine_blackboard (cast `/Game/AI/StateMachine/BP_StateMachine_Blackboard` (`RpStateMachineComponent.StateMachineBlackboard` (`self.State Machine`))))
      (`|ExecutionSequence`
        (:`then_0`
          (`/Game/AI/StateMachine/BP_StateMachine_Blackboard.SetAgent` _asbp_state_machine_blackboard (`self.K2_GetPawn`)))
        (:`then_1`
          (`/Game/AI/StateMachine/BP_StateMachine_Blackboard.SetController` _asbp_state_machine_blackboard self))))
    (:`then_1`
      (`RpStateMachineComponent.Start` (`self.State Machine`)))))

(fn `UserConstructionScript`)