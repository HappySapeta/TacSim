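; BP_Player_Controller is a player controller that handles Enhanced Input for moving and looking.
; BeginPlay adds the IMC_Default mapping context to the local player subsystem.
; IA_Move drives movement input on player pawn 0 along its forward and right vectors, while IA_Look feeds pitch and yaw input to the controller.
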(event `self.ReceiveBeginPlay`
  (`EnhancedInputSubsystemInterface.AddMappingContext` (subsystem `EnhancedInputLocalPlayerSubsystem`) "/Game/GameManagement/IMC_Default.IMC_Default" 0 (struct)))

(event `EnhancedInput|/Game/GameManagement/IA_Move`
  (params (ActionValue :type "Vector2D Structure") (ElapsedSeconds :type "Float (double-precision)") (TriggeredSeconds :type "Float (double-precision)") (InputAction :type "InputAction Object Reference" :default "/Game/GameManagement/IA_Move.IA_Move"))
  (bind _returnvalue (`GameplayStatics.GetPlayerPawn` 0))
  (bind (_x _y) (`KismetMathLibrary.BreakVector2D` ActionValue))
  (:`Triggered`
    (`Pawn.AddMovementInput` _returnvalue (+ (* _y (`self.GetActorForwardVector` _returnvalue)) (* _x (`self.GetActorRightVector` _returnvalue))) 1.0 false)))

(event `EnhancedInput|/Game/GameManagement/IA_Look`
  (params (ActionValue :type "Vector2D Structure") (ElapsedSeconds :type "Float (double-precision)") (TriggeredSeconds :type "Float (double-precision)") (InputAction :type "InputAction Object Reference" :default "/Game/GameManagement/IA_Look.IA_Look"))
  (bind (_x _y) (`KismetMathLibrary.BreakVector2D` ActionValue))
  (:`Triggered`
    (`self.AddPitchInput` _y)
    (`self.AddYawInput` _x)))

(fn `UserConstructionScript`)