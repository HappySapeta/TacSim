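; BP_State_Patrol is an AI state machine state that sends the agent to a random nearby point when activated.
; The destination is a random direction scaled between the min and max patrol range from the agent's location, keeping its current Z.
; AI MoveTo uses the controller and agent from the state machine blackboard, whose IsPatrolling flag is set during the move and cleared on success or failure.
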(event `self.OnActivate`
  (bind _returnvalue (`self.GetContext` "/Game/AI/StateMachine/BP_StateMachine_Blackboard.BP_StateMachine_Blackboard_C"))
  (bind _returnvalue_2 (`self.GetContext` "/Game/AI/StateMachine/BP_StateMachine_Blackboard.BP_StateMachine_Blackboard_C"))
  (bind _pawn (`/Game/AI/StateMachine/BP_StateMachine_Blackboard.GetAgent` _returnvalue))
  (bind _returnvalue_3 (`Actor.K2_GetActorLocation` _pawn))
  (`parent.OnActivate`)
  (`|AIMoveTo` (`/Game/AI/StateMachine/BP_StateMachine_Blackboard.GetController` _returnvalue) _pawn (`KismetMathLibrary.MakeVector` (.x (+ _returnvalue_3 (* (`KismetMathLibrary.RandomUnitVector`) (`KismetMathLibrary.RandomFloatInRange` (`self.MinPatrolRange`) (`self.MaxPatrolRange`))))) (.y (+ _returnvalue_3 (* (`KismetMathLibrary.RandomUnitVector`) (`KismetMathLibrary.RandomFloatInRange` (`self.MinPatrolRange`) (`self.MaxPatrolRange`))))) (.z _returnvalue_3)) null
    (:`then`
      (set `/Game/AI/StateMachine/BP_StateMachine_Blackboard.IsPatrolling` true _returnvalue_2))
    (:`OnSuccess`
      (set `/Game/AI/StateMachine/BP_StateMachine_Blackboard.IsPatrolling` false _returnvalue_2 :!label _label))
    (:`OnFail`
      (goto _label))))