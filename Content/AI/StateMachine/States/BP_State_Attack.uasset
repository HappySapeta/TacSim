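; Attack state for an AI state machine that keeps the agent facing its attack target.
; On each state update it reads the AttackTarget from the state machine blackboard context and, if valid, snaps the agent's rotation to look directly at it.
; Activation and deactivation only call the parent, and the state itself triggers no attack action.
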(event `self.OnActivate`
  (`parent.OnActivate`))

(event `self.OnDeactivate`
  (`parent.OnDeactivate`))

(event `self.StateUpdate`
  (params (DeltaTime :type "Float (single-precision)"))
  (bind _returnvalue (`self.GetContext` "/Game/AI/StateMachine/BP_StateMachine_Blackboard.BP_StateMachine_Blackboard_C"))
  (bind _pawn (`/Game/AI/StateMachine/BP_StateMachine_Blackboard.GetAgent` _returnvalue))
  (bind _attacktarget (`/Game/AI/StateMachine/BP_StateMachine_Blackboard.AttackTarget` _returnvalue))
  (`/Engine/EditorBlueprintResources/StandardMacros.IsValid` _attacktarget
    (:`Is Valid`
      (`Actor.K2_SetActorRotation` _pawn (`KismetMathLibrary.FindLookAtRotation` (`Actor.K2_GetActorLocation` _pawn) (`Actor.K2_GetActorLocation` _attacktarget)) false))))