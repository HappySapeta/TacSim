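; GOAP action that moves an AI agent to the blackboard's GoToLocation.
; On perform it runs AIMoveTo and completes the action only on success, with no failure branch wired.
; Simulate predicts the result by setting the CurrentLocation fact to the goal location.
; ApplyEffects instead writes the agent's actual position to that fact in the target state, both as instanced-struct vector variants.
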(event `self.BP_OnPerformAction`
  (bind _returnvalue (`self.GetContext` "/Game/AI/GOAP/BP_GOAP_Blackboard.BP_GOAP_Blackboard_C"))
  (`|AIMoveTo` (`/Game/AI/GOAP/BP_GOAP_Blackboard.GetController` _returnvalue) (`/Game/AI/GOAP/BP_GOAP_Blackboard.GetAgent` _returnvalue) (`/Game/AI/GOAP/BP_GOAP_Blackboard.GoToLocation` _returnvalue) null
    (:`OnSuccess`
      (`self.OnActionComplete`))))

(event `self.ApplyEffects`
  (bind _returnvalue (`BlueprintInstancedStructLibrary.MakeInstancedStruct` (make `RpVariantVector3` (`Actor.K2_GetActorLocation` (`/Game/AI/GOAP/BP_GOAP_Blackboard.GetAgent` (`self.GetContext` "/Game/AI/GOAP/BP_GOAP_Blackboard.BP_GOAP_Blackboard_C"))))))
  (`RpGOAPState.SetFact` (`self.TargetState`) (`BlueprintGameplayTagLibrary.MakeLiteralGameplayTag` (struct :`TagName` "GOAP.PlayerState.CurrentLocation")) (make `RpStateDescriptor` _returnvalue)))

(fn `Simulate`
  (params (Current :type "RpGOAPState Object Reference"))
  (bind _returnvalue (`BlueprintInstancedStructLibrary.MakeInstancedStruct` (make `RpVariantVector3` (`/Game/AI/GOAP/BP_GOAP_Blackboard.GoToLocation` (`self.GetContext` "/Game/AI/GOAP/BP_GOAP_Blackboard.BP_GOAP_Blackboard_C")))))
  (`RpGOAPState.SetFact` Current (`BlueprintGameplayTagLibrary.MakeLiteralGameplayTag` (struct :`TagName` "GOAP.PlayerState.CurrentLocation")) (make `RpStateDescriptor` _returnvalue))
  (return))