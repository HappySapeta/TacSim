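; BP_GOAP_Actor is a test actor that exercises the RpGOAP planner when the F key is pressed.
; It constructs a BP_GOAP_StartingState and a BP_GOAP_TestAction, then passes both to the planner's Simulate call.
; The resulting state is stored in NewState, with no further use of it in the graph.
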(event `Key|F`
  (params (Key :type "Key Structure"))
  (:`Pressed`
    (bind _returnvalue (`RpGOAPComponent.GetPlanner` (`self.RpGOAP`)))
    (`|ExecutionSequence`
      (:`then_0`
        (bind _returnvalue_2 (`|GenericCreateObject` "/Game/Test/GOAP/BP_GOAP_StartingState.BP_GOAP_StartingState_C"))
        (set `self.State` _returnvalue_2))
      (:`then_1`
        (bind _returnvalue_3 (`|GenericCreateObject` "/Game/Test/GOAP/BP_GOAP_TestAction.BP_GOAP_TestAction_C"))
        (set `self.Action` _returnvalue_3))
      (:`then_2`
        (bind _returnvalue_4 (`RpGOAPPlanner.Simulate` _returnvalue (`self.State`) (`self.Action`)))
        (set `self.NewState` _returnvalue_4)))))

(fn `UserConstructionScript`)