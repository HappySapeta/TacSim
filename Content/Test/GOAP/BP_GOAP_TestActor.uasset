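; BP_GOAP_TestActor is a test actor that checks GOAP goal evaluation against a world state.
; On BeginPlay it constructs a BP_GOAP_Goal and a BP_GOAP_State and stores them.
; Pressing F evaluates the goal against that state and prints whether the evaluation succeeded.
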(event `self.ReceiveBeginPlay`
  (bind _returnvalue (`|GenericCreateObject` "/Game/Test/GOAP/BP_GOAP_Goal.BP_GOAP_Goal_C"))
  (set `self.GoalState` _returnvalue)
  (bind _returnvalue_2 (`|GenericCreateObject` "/Game/Test/GOAP/BP_GOAP_State.BP_GOAP_State_C"))
  (set `self.TestState` _returnvalue_2))

(event `Key|F`
  (params (Key :type "Key Structure"))
  (:`Pressed`
    (bind _returnvalue (`RpGOAPGoalState.Evaluate` (`self.GoalState`) (`self.TestState`)))
    (if _returnvalue
      (`KismetSystemLibrary.PrintString` "Evaluation successful!" true true (struct :`R` 0.001879 :`G` 1.0 :`B` 0.041556 :`A` 1.0))
      (else
        (`KismetSystemLibrary.PrintString` "Evaluation unsuccessful!" true true (struct :`R` 1.0 :`G` 0.022299 :`B` 0.000498 :`A` 1.0))))))

(fn `UserConstructionScript`)